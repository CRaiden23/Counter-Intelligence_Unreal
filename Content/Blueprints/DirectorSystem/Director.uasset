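; Director that lets Twitch chat vote on gameplay events affecting the player and guards.
; After IRC authentication, timers cycle voting rounds: it draws up to three distinct random events, announces them in chat and counts one numbered vote per user.
; The winner, or a random option if none has votes, runs through an enum switch.
; Only the noise at the player and guard patrol shuffle are implemented; other events print "Unimplemented".
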(event OnMessageReceived(TwitchIRC)
  (params (Message :type String) (User :type String))
  (bind _returnvalue (Math|Conversions|ToInteger(Byte) Message))
  (bind _vote_buckets (Variables|VotingSystem|GetVote%20Buckets))
  (bind _returnvalue_2 (- _returnvalue 1))
  (if (Variables|VotingSystem|GetListening%20For%20Votes)
    ;[1 1 1] Ignore Users Who Already Voted
    (if (not (Utilities|Set|Contains (Variables|VotingSystem|GetVoters) User))
      (if (and (> _returnvalue 0) (<= _returnvalue (Utilities|Array|Length (Variables|VotingSystem|GetVote%20Buckets))))
        (Utilities|Array|SetArrayElem _vote_buckets _returnvalue_2 (+ (Utilities|Array|Get(acopy) _vote_buckets _returnvalue_2) 1))
        (Utilities|Set|Add (Variables|VotingSystem|GetVoters) User)))))

(event OnAuthentication(TwitchIRC)
  (Utilities|Time|SetTimerbyEvent (delegate Custom|Begin%20Listening%20for%20Votes) 15.0))

(event Custom|Begin%20Listening%20for%20Votes
  (bind _events_set (VotingSystem|SelectEventstoVoteon))
  (if _events_set
    (VotingSystem|AnnounceVoting)
    (Development|PrintString "Listening for Votes!" true true "(R=1.000000,G=0.000000,B=0.258183,A=1.000000)" 5.0)
    (Variables|VotingSystem|SetListening%20For%20Votes true)
    (Utilities|Time|SetTimerbyEvent (delegate Custom|Stop%20Listening%20for%20Votes) 3e+01)
    (else
      (Variables|VotingSystem|SetListening%20For%20Votes false))))

(event Custom|Stop%20Listening%20for%20Votes
  (bind _twitchirc (Variables|Default|GetTwitchIRC))
  (Utilities|FlowControl|Sequence
    (:then_0
      ;[1 1 1] Stop Listening, Set Winner
      (Development|PrintString "Voting Ended!" true true "(R=1.000000,G=0.000000,B=0.259243,A=1.000000)" 5.0)
      (bind _winning_event (VotingSystem|GetWinningEvent))
      (bind _output_get (Variables|VotingSystem|SetWinning%20Event _winning_event))
      (Variables|VotingSystem|SetListening%20For%20Votes false)
      (Utilities|Array|Clear (Variables|VotingSystem|GetVote%20Buckets))
      (Utilities|Array|Clear (Variables|VotingSystem|GetEvents%20To%20Be%20Voted%20On))
      (Utilities|Set|Clear (Variables|VotingSystem|GetVoters))
      (Class|TwitchIRCComponent|SendtoChat _twitchirc (Utilities|String|Append "Voting has ended! " (Utilities|String|Append "\"" (Utilities|String|EnumtoString _output_get) "\" Wins!")) (Variables|/Script/Counter_Intelligence.TwitchIRCComponent|GetChannelName _twitchirc)))
    (:then_1
      ;[1 1 1] Execute Winning Event
      (DirectorEvents|ExecuteDirectorEvent)
      (Utilities|Time|SetTimerbyEvent (delegate Custom|Begin%20Listening%20for%20Votes) 10.5 false 5.5 15.0))))

(fn ConstructionScript)

(fn AnnounceVoting
  (bind _twitchirc (Variables|Default|GetTwitchIRC))
  (bind _twitchirc_2 (Variables|Default|GetTwitchIRC))
  (Class|TwitchIRCComponent|SendtoChat _twitchirc_2 "Voting has begun!" (Variables|/Script/Counter_Intelligence.TwitchIRCComponent|GetChannelName _twitchirc_2))
  (for (_array_element _array_index) (Variables|VotingSystem|GetEvents%20To%20Be%20Voted%20On)
    (Class|TwitchIRCComponent|SendtoChat _twitchirc (Utilities|String|Append (Utilities|String|ToString(Integer) (+ _array_index 1)) ": " (Utilities|String|EnumtoString _array_element) " 
") (Variables|/Script/Counter_Intelligence.TwitchIRCComponent|GetChannelName _twitchirc))))

(fn SelectEventstoVoteon
  (bind _numberofevents (LocalVariables|GetNumberOfEvents))
  (bind _returnvalue (Math|Conversions|ToInteger(Byte) _numberofevents))
  (bind _returnvalue_2 (- _returnvalue 1))
  ;[1 1 1] Fail Out If We Have Nothing To Vote For
  (if (!= _returnvalue 0)
    (for _index (range 0 (Math|Integer|Clamp(Integer) 2 0 _returnvalue_2))
      (bind _output_get (LocalVariables|SetRandIndex (Math|Random|RandomIntegerinRange 0 _returnvalue_2)))
      ;[1 1 1] Increment Random Number if we have already used it
      (while (Utilities|Set|Contains (LocalVariables|GetIndicesUsed) _output_get)
        (LocalVariables|SetRandIndex (Math|Integer|%(Integer) (+ (LocalVariables|GetRandIndex) 1) (Math|Conversions|ToInteger(Byte) (LocalVariables|GetNumberOfEvents)))))
      ;[1 1 1] Mark Index as used
      (Utilities|Set|Add (LocalVariables|GetIndicesUsed) (LocalVariables|GetRandIndex))
      ;[1 1 1] Add Event to our Voting Array
      (Utilities|Array|Add (Variables|VotingSystem|GetEvents%20To%20Be%20Voted%20On) (Utilities|Enum|ByteToEnumDirectorEvents_Enum (Math|Conversions|ToByte(Integer) (LocalVariables|GetRandIndex)))))
    ;[1 1 1] Resize Vote Buckets Appropriately
    (Utilities|Array|Resize (Variables|VotingSystem|GetVote%20Buckets) (Utilities|Array|Length (Variables|VotingSystem|GetEvents%20To%20Be%20Voted%20On)))
    (return true)
    (else
      (return false))))

(fn GetWinningEvent
  ;[1 1 1] Find the Winning Index
  (for (_array_element _array_index) (Variables|VotingSystem|GetVote%20Buckets)
    (if (> _array_element (LocalVariables|GetMax%20Votes))
      (LocalVariables|SetMax%20Votes _array_element)
      (LocalVariables|SetWinning%20Index _array_index)))
  (if (== (LocalVariables|GetWinning%20Index) -1)
    ;[1 1 1] 3-Way Tie
    (return (Utilities|Array|Get(acopy) (Variables|VotingSystem|GetEvents%20To%20Be%20Voted%20On) (Math|Random|RandomIntegerinRange 0 (- (Utilities|Array|Length (Variables|VotingSystem|GetEvents%20To%20Be%20Voted%20On)) 1))))
    (else
      (return (Utilities|Array|Get(acopy) (Variables|VotingSystem|GetEvents%20To%20Be%20Voted%20On) (LocalVariables|GetWinning%20Index))))))

(fn ExecuteDirectorEvent
  (bind _returnvalue (Game|GetPlayerCharacter 0))
  (switch Utilities|FlowControl|Switch|SwitchonDirectorEvents_Enum (Variables|VotingSystem|GetWinning%20Event)
    (:NewEnumerator1
      (Class|AISenseHearing|ReportNoiseEvent (Transformation|GetActorLocation _returnvalue) 1.0 _returnvalue 0.0 "Director")
      (Development|PrintString "Sound played on player"))
    (:NewEnumerator2
      (Development|PrintString "Unimplemented" true true "(R=0.000000,G=0.000000,B=0.000000,A=1.000000)" 1e+01 :!label _label))
    (:NewEnumerator4
      (goto _label))
    (:NewEnumerator5
      (goto _label))
    (:NewEnumerator6
      (goto _label))
    (:NewEnumerator7
      (goto _label))
    (:NewEnumerator8
      (bind _outactors (Actor|GetAllActorsOfClass "/Game/Blueprints/Enemies/ALS_Guard_CharacterBP.ALS_Guard_CharacterBP_C"))
      (bind _output_get (LocalVariables|SetGuard%20Array _outactors))
      (for _array_element _output_get
        (Utilities|IsValid (Actor|GetComponentbyClass _array_element "/Game/Blueprints/Enemies/AIPatrol_ABP.AIPatrol_ABP_C")
          (:Is%20Valid
            (Default|PopulatePatrolRoute (Actor|GetComponentbyClass _array_element "/Game/Blueprints/Enemies/AIPatrol_ABP.AIPatrol_ABP_C")))))
      (Development|PrintString "All Guard Patrols Shuffled"))))