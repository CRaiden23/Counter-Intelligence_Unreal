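; Electric floor hazard that shocks an actor standing in its box trigger while it is active.
; Box overlap stores the latest actor and opens a gate, and end overlap clears it and closes the gate.
; Tick passes through the gate once the damage cooldown has elapsed, applying fixed damage and resetting the timer.
; Activate and Deactivate toggle the hazard along with its Niagara lightning aura and looping-style audio cue.
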(event OnComponentEndOverlap(Box)
  (params (OverlappedComponent :type Primitive%20Component%20Object%20Reference) (OtherActor :type Actor%20Object%20Reference) (OtherComp :type Primitive%20Component%20Object%20Reference) (OtherBodyIndex :type Integer))
  (Variables|Default|SetOverlap%20Actor 0)
  (Utilities|FlowControl|Gate true) ; enters at Close
)

(event OnComponentBeginOverlap(Box)
  (params (OverlappedComponent :type Primitive%20Component%20Object%20Reference) (OtherActor :type Actor%20Object%20Reference) (OtherComp :type Primitive%20Component%20Object%20Reference) (OtherBodyIndex :type Integer) (bFromSweep :type Boolean) (SweepResult :type Hit%20Result%20Structure%20%28by%20ref%29))
  (Variables|Default|SetOverlap%20Actor OtherActor)
  (Utilities|FlowControl|Gate true) ; enters at Open
)

(event EventTick
  (params (DeltaSeconds :type Float%20%28single-precision%29))
  (if (and (> (Math|Float|Absolute(Float) (- (Utilities|Time|GetTimeSeconds) (Variables|Default|GetLastDamageTime))) (Variables|Default|GetDamageCooldownTime)) (Variables|Default|GetisActive))
    (Utilities|FlowControl|Gate true
      (:Exit
        (bind _overlap_actor (Variables|Default|GetOverlap%20Actor)
          (:then
            (Variables|Default|SetLastDamageTime (Utilities|Time|GetTimeSeconds))
            (Game|Damage|ApplyDamage _overlap_actor 15.0 0 0))
          (:else))))))

(event EventActivate
  (bind _output_get (Variables|Default|SetisActive true))
  (Components|Activation|SetActive (Variables|Default|GetNS_LightningAura_1) _output_get false)
  (Audio|Components|Audio|Play (Variables|Default|GetAudioCue) 0.0))

(event EventDeactivate
  (bind _output_get (Variables|Default|SetisActive false))
  (Components|Activation|SetActive (Variables|Default|GetNS_LightningAura_1) _output_get false)
  (Audio|Components|Audio|Stop (Variables|Default|GetAudioCue)))

(fn ConstructionScript)