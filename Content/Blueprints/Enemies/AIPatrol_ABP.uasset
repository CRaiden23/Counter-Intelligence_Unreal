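; Enemy AI patrol Blueprint that holds a route of patrol points and supplies the next location to move to.
; On BeginPlay, an empty route is filled from the level's shuffled TargetPoint actors, with a random length of up to four, possibly none.
; FindNextPatrolPoint returns the current point's location and advances the index, either looping or ping-ponging through a Flipped flag, falling back to the first point if invalid.
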(event EventBeginPlay
  (if (== (Utilities|Array|Length (Variables|Default|GetPatrolPoints)) 0)
    (CallFunction|PopulatePatrolRoute)))

(event EventTick
  (params (DeltaSeconds :type Float%20%28single-precision%29)))

(fn FindNextPatrolPoint
  (params (Cycle :type Boolean))
  (LocalVariables|SetNext%20Patrol%20Point (Utilities|Array|Get(acopy) (Variables|Default|GetPatrolPoints) (Variables|Default|GetCurrent%20Patrol%20Point)))
  (if Cycle
    ;[1 1 1] Cyclic Patrol
    (if (== (Variables|Default|GetCurrent%20Patrol%20Point) (Utilities|Array|LastIndex (Variables|Default|GetPatrolPoints)))
      (Variables|Default|SetCurrent%20Patrol%20Point 0)
      (else
        (Variables|Default|SetCurrent%20Patrol%20Point (+ (Variables|Default|GetCurrent%20Patrol%20Point) 1))))
    (else
      ;[1 1 1] Acyclic Patrol
      (if (Variables|Default|GetFlipped)
        ;;[1 1 1] Reversed
        (Variables|Default|SetCurrent%20Patrol%20Point (- (Variables|Default|GetCurrent%20Patrol%20Point) 1))
        (if (== (Variables|Default|GetCurrent%20Patrol%20Point) 0) ; Reverse if at the beginning
          (Variables|Default|SetFlipped false))
        (else
          ;;[1 1 1] Normal
          (Variables|Default|SetCurrent%20Patrol%20Point (+ (Variables|Default|GetCurrent%20Patrol%20Point) 1))
          (if (== (Variables|Default|GetCurrent%20Patrol%20Point) (Utilities|Array|LastIndex (Variables|Default|GetPatrolPoints))) ; Reverse if at the end
            (Variables|Default|SetFlipped true))))))
  (Variables|Default|SetCurrent%20Patrol%20Point (Math|Integer|Clamp(Integer) (Variables|Default|GetCurrent%20Patrol%20Point) 0 (- (Utilities|Array|Length (Variables|Default|GetPatrolPoints)) 1)))
  (Utilities|IsValid (LocalVariables|GetNext%20Patrol%20Point)
    (:Is%20Valid
      (return (Transformation|GetActorLocation (LocalVariables|GetNext%20Patrol%20Point))))
    (:Is%20Not%20Valid
      (return (Transformation|GetActorLocation (Utilities|Array|Get(acopy) (Variables|Default|GetPatrolPoints)))))))

(fn PopulatePatrolRoute
  (Utilities|Array|Clear (Variables|Default|GetPatrolPoints))
  (bind _outactors (Actor|GetAllActorsOfClass "/Script/Engine.TargetPoint"))
  (bind _output_get (LocalVariables|SetAllPossiblePatrolPoints _outactors))
  (Utilities|Array|Shuffle _output_get)
  (bind _output_get_2 (LocalVariables|SetPatrol%20Route%20Length (Math|Random|RandomIntegerinRange 0 4)))
  (for (_array_element _array_index) _output_get
    (if (== _array_index _output_get_2)
      (return)
      (else
        (Utilities|Array|Add (Variables|Default|GetPatrolPoints) _array_element))))
  (return))