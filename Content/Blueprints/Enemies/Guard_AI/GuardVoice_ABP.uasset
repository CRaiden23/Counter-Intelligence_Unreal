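; Guard voice Blueprint that supplies random bark lines for enemy guard AI.
; Each function picks a random entry from one category of GuardVoiceBox, covering suspicion, alert, injury, death, chatter, backup calls and player kills.
; Despite their Play names, the functions only return the selected line and leave playback to the caller.
; The event graph holds no active logic.
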(event EventBeginPlay)

(event EventTick
  (params (DeltaSeconds :type Float%20%28single-precision%29)))

(fn PlaySuspiciousLine
  (return (.OutItem (Utilities|Array|Random (.Suspicion (Utilities|Struct|BreakGuardVoiceBox_Struct (Variables|Default|GetGuardVoiceBox)))))))

(fn PlayAlertLine
  (return (.OutItem (Utilities|Array|Random (.Alert (Utilities|Struct|BreakGuardVoiceBox_Struct (Variables|Default|GetGuardVoiceBox)))))))

(fn PlayInjuredLine
  (return (.OutItem (Utilities|Array|Random (.Injured (Utilities|Struct|BreakGuardVoiceBox_Struct (Variables|Default|GetGuardVoiceBox)))))))

(fn PlayDeathLine
  (return (.OutItem (Utilities|Array|Random (.Death (Utilities|Struct|BreakGuardVoiceBox_Struct (Variables|Default|GetGuardVoiceBox)))))))

(fn PlayChatterLine
  (return (.OutItem (Utilities|Array|Random (.Chatter (Utilities|Struct|BreakGuardVoiceBox_Struct (Variables|Default|GetGuardVoiceBox)))))))

(fn PlayBackupLine
  (return (.OutItem (Utilities|Array|Random (.NeedBackup (Utilities|Struct|BreakGuardVoiceBox_Struct (Variables|Default|GetGuardVoiceBox)))))))

(fn PlayPlayerKillLine
  (return (.OutItem (Utilities|Array|Random (.PlayerKilled (Utilities|Struct|BreakGuardVoiceBox_Struct (Variables|Default|GetGuardVoiceBox)))))))