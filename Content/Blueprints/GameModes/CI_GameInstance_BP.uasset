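; Game instance that holds the player's loadout, ammo caps and starting amounts, health and stealth modifiers, upgrade token balance and Twitch login details.
; Update functions clamp numeric changes or swap equipment by slot, returning a bool intended to signal whether the value changed.
; Getters expose the loadout and ammo, granting starting amounts only for filled slots, with either item count or battery charge depending on the special.
; ResetSettings restores loadout, stats and tokens to defaults.
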(fn UpdateStealthMod
  (params (Delta :type Float%20%28single-precision%29))
  (LocalVariables|SetOriginal%20Value (Variables|PlayerModifiers|GetStealthModifier))
  (Variables|PlayerModifiers|SetStealthModifier (Math|Float|Clamp(Float) (+ Delta (Variables|PlayerModifiers|GetStealthModifier)) 0.5 1.5))
  (return (!= (Math|Float|Clamp(Float) (+ Delta (Variables|PlayerModifiers|GetStealthModifier)) 0.5 1.5) (LocalVariables|GetOriginal%20Value))))

(fn UpdatePrimaryCap
  (params (Delta :type Integer))
  (LocalVariables|SetOriginal%20Value (Variables|PlayerLoadout|GetPrimaryAmmoCap))
  (Variables|PlayerLoadout|SetPrimaryAmmoCap (Math|Integer|Clamp(Integer) (+ Delta (Variables|PlayerLoadout|GetPrimaryAmmoCap)) 32 128))
  (return (!= (Math|Integer|Clamp(Integer) (+ Delta (Variables|PlayerLoadout|GetPrimaryAmmoCap)) 32 128) (LocalVariables|GetOriginal%20Value))))

(fn UpdateSecondaryCap
  (params (Delta :type Integer))
  (LocalVariables|SetOriginal%20Value (Variables|PlayerLoadout|GetSecondaryAmmoCap))
  (Variables|PlayerLoadout|SetSecondaryAmmoCap (Math|Integer|Clamp(Integer) (+ Delta (Variables|PlayerLoadout|GetSecondaryAmmoCap)) 16 64))
  (return (!= (Math|Integer|Clamp(Integer) (+ Delta (Variables|PlayerLoadout|GetSecondaryAmmoCap)) 16 64) (LocalVariables|GetOriginal%20Value))))

(fn UpdateEquipment
  (params (Equipment%20Type :type E_PickupType%20Enum :default "NewEnumerator0") (Weapon :type Weapon%20BP%20Class%20Reference) (New%20Throwable :type Throwable%20BP%20Class%20Reference) (New%20Special :type Specials%20Enum :default "NewEnumerator5"))
  (switch Utilities|FlowControl|Switch|SwitchonE_PickupType Equipment%20Type
    (:NewEnumerator0
      (bind _output_get (LocalVariables|SetSuccess (!= (Variables|PlayerLoadout|GetPrimaryWeapon) Weapon)))
      (if _output_get
        (Variables|PlayerLoadout|SetPrimaryWeapon Weapon))
      (return (LocalVariables|GetSuccess)))
    (:NewEnumerator1
      (bind _output_get_2 (LocalVariables|SetSuccess (!= (Variables|PlayerLoadout|GetSecondaryWeapon) Weapon)))
      (if _output_get_2
        (Variables|PlayerLoadout|SetSecondaryWeapon Weapon))
      (return (LocalVariables|GetSuccess)))
    (:NewEnumerator2
      (bind _output_get_3 (LocalVariables|SetSuccess (!= New%20Throwable (Variables|PlayerLoadout|GetThrowable))))
      (if _output_get_3
        (Variables|PlayerLoadout|SetThrowable New%20Throwable))
      (return (LocalVariables|GetSuccess)))
    (:NewEnumerator3
      (bind _output_get_4 (LocalVariables|SetSuccess (Utilities|Enum|NotEqual(Enum) New%20Special (Variables|PlayerLoadout|GetSpecial))))
      (if _output_get_4
        (Variables|PlayerLoadout|SetSpecial New%20Special))
      (return (LocalVariables|GetSuccess)))))

(fn UpdateHealthCap
  (params (Delta :type Float%20%28single-precision%29))
  (LocalVariables|SetOriginal%20Value (Variables|PlayerModifiers|GetHealthModifier))
  (Variables|PlayerModifiers|SetHealthModifier (Math|Float|Clamp(Float) (+ Delta (Variables|PlayerModifiers|GetHealthModifier)) 0.5 2.0))
  (return (!= (Math|Float|Clamp(Float) (+ Delta (Variables|PlayerModifiers|GetHealthModifier)) 0.5 2.0) (LocalVariables|GetOriginal%20Value))))

(fn NTokensAvailable?
  (params (Number%20of%20Tokens :type Integer))
  (return (>= (Variables|Tokens|GetTokens%20Available) Number%20of%20Tokens)))

(fn UpdateTokensAvailable
  (params (Delta :type Integer))
  (LocalVariables|SetOriginal%20Value (Variables|Tokens|GetTokens%20Available))
  (Variables|Tokens|SetTokens%20Available (Math|Integer|Clamp(Integer) (+ Delta (Variables|Tokens|GetTokens%20Available)) 0 99))
  (return (!= (Math|Integer|Clamp(Integer) (+ Delta (Variables|Tokens|GetTokens%20Available)) 0 99) (LocalVariables|GetOriginal%20Value))))

(fn SetTwitchInfo
  (params (Twitch%20OAuth :type String) (Twitch%20Username :type String) (Twitch%20Channel :type String))
  (Variables|Twitch|SetTwitch%20OAuth Twitch%20OAuth)
  (Variables|Twitch|SetTwitch%20Username Twitch%20Username)
  (Variables|Twitch|SetTwitch%20Channel Twitch%20Channel)
  (Variables|Twitch|SetTwitch%20Setup true))

(fn GetStartingAmmo
  (Utilities|FlowControl|Sequence
    (:then_0
      (Variables|PlayerLoadout|GetPrimaryWeapon
        (:then
          (LocalVariables|SetResulting%20Primary%20Ammo (Variables|PlayerLoadout|GetStartingPrimaryAmmo)))
        (:else)))
    (:then_1
      (Variables|PlayerLoadout|GetSecondaryWeapon
        (:then
          (LocalVariables|SetResulting%20Secondary%20Ammo (Variables|PlayerLoadout|GetStartingSecondaryAmmo)))
        (:else)))
    (:then_2
      (Variables|PlayerLoadout|GetThrowable
        (:then
          (LocalVariables|SetResulting%20Throwable%20Ammo (Variables|PlayerLoadout|GetStartingGrenadeAmmo)))
        (:else)))
    (:then_3
      (switch Utilities|FlowControl|Switch|SwitchonSpecials (Variables|PlayerLoadout|GetSpecial)
        (:NewEnumerator0
          (LocalVariables|SetResulting%20Equipment%20Count (Variables|PlayerLoadout|GetStartingEquipmentCount) :!label _label))
        (:NewEnumerator1
          (LocalVariables|SetResulting%20Battery%20Charge (Variables|PlayerLoadout|GetStartingBatteryCharge) :!label _label_2))
        (:NewEnumerator2
          (goto _label_2))
        (:NewEnumerator3
          (goto _label_2))
        (:NewEnumerator6
          (goto _label))))
    (:then_4
      (return (LocalVariables|GetResulting%20Primary%20Ammo) (LocalVariables|GetResulting%20Secondary%20Ammo) (LocalVariables|GetResulting%20Throwable%20Ammo) (LocalVariables|GetResulting%20Equipment%20Count) (LocalVariables|GetResulting%20Battery%20Charge)))))

(fn UpdateStartingAmmo
  (params (Equipment :type E_PickupType%20Enum :default "NewEnumerator0") (Delta :type Integer))
  (switch Utilities|FlowControl|Switch|SwitchonE_PickupType Equipment
    (:NewEnumerator0
      (LocalVariables|SetOriginal%20Value (Variables|PlayerLoadout|GetStartingPrimaryAmmo))
      (Variables|PlayerLoadout|SetStartingPrimaryAmmo (Math|Integer|Clamp(Integer) (+ Delta (Variables|PlayerLoadout|GetStartingPrimaryAmmo)) 0 128))
      (return (!= (Math|Integer|Clamp(Integer) (+ Delta (Variables|PlayerLoadout|GetStartingPrimaryAmmo)) 0 128) (LocalVariables|GetOriginal%20Value))))
    (:NewEnumerator1
      (LocalVariables|SetOriginal%20Value (Variables|PlayerLoadout|GetStartingSecondaryAmmo))
      (Variables|PlayerLoadout|SetStartingSecondaryAmmo (Math|Integer|Clamp(Integer) (+ Delta (Variables|PlayerLoadout|GetStartingSecondaryAmmo)) 0 64))
      (return (!= (Math|Integer|Clamp(Integer) (+ Delta (Variables|PlayerLoadout|GetStartingSecondaryAmmo)) 0 64) (LocalVariables|GetOriginal%20Value))))))

(fn GetMaxAmmo
  (return (Variables|PlayerLoadout|GetPrimaryAmmoCap) (Variables|PlayerLoadout|GetSecondaryAmmoCap) (Variables|PlayerLoadout|GetGrenadeAmmoCap)))

(fn GetStartingLoadout
  (return (Variables|PlayerLoadout|GetPrimaryWeapon) (Variables|PlayerLoadout|GetSecondaryWeapon) (Variables|PlayerLoadout|GetThrowable) (Variables|PlayerLoadout|GetSpecial)))

(fn ResetSettings
  (Variables|PlayerLoadout|SetPrimaryWeapon 0)
  (Variables|PlayerLoadout|SetPrimaryAmmoCap 64)
  (Variables|PlayerLoadout|SetStartingPrimaryAmmo 32)
  (Variables|PlayerLoadout|SetSecondaryWeapon 0)
  (Variables|PlayerLoadout|SetSecondaryAmmoCap 32)
  (Variables|PlayerLoadout|SetStartingSecondaryAmmo 16)
  (Variables|PlayerLoadout|SetThrowable 0)
  (Variables|PlayerLoadout|SetGrenadeAmmoCap 2)
  (Variables|PlayerLoadout|SetStartingGrenadeAmmo 0)
  (Variables|PlayerLoadout|SetSpecial "NewEnumerator5")
  (Variables|PlayerLoadout|SetStartingEquipmentCount 0)
  (Variables|PlayerLoadout|SetStartingBatteryCharge 1e+02)
  (Variables|PlayerModifiers|SetHealthModifier 1.0)
  (Variables|PlayerModifiers|SetStealthModifier 1.0)
  (Variables|Tokens|SetTokens%20Available (Variables|Tokens|GetStartingTokens)))