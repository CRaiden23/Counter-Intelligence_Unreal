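; Game state Blueprint that drives adaptive music intensity based on how many enemies are alerted.
; ChangeMusicState sets a target state and raises or lowers the alerted-enemy count, while ResetMusicState clears the count.
; Tick eases the current state toward the target and feeds it to the music cue's State parameter, holding any decrease until no alerted enemies remain.
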(event EventBeginPlay)

(event EventTick
  (params (DeltaSeconds :type Float%20%28single-precision%29))
  (if (> (Math|Float|Absolute(Float) (- (Variables|Default|GetTarget%20State) (Variables|Default|GetMusic%20State))) 0.0)
    (bind _output_get (Variables|Default|SetMusic%20State (Math|Float|Lerp (Variables|Default|GetMusic%20State) (Variables|Default|GetTarget%20State) (select (and (< (Variables|Default|GetTarget%20State) (Variables|Default|GetMusic%20State)) (!= (Variables|Default|GetAlert%20Enemies) 0)) 0.0 0.02))))
    (Audio|Parameter|SetFloatParameter (Variables|Default|GetMusic_Cue) "State" _output_get :!class /Script/Engine.AudioComponent)))

(event EventChangeMusicState
  (params (MusicState :type Float%20%28single-precision%29))
  (bind _output_get (Variables|Default|SetTarget%20State MusicState))
  (if (> _output_get 0.5)
    (Variables|Default|SetAlert%20Enemies (+ (Variables|Default|GetAlert%20Enemies) 1))
    (else
      (Variables|Default|SetAlert%20Enemies (Math|Integer|Clamp(Integer) (- (Variables|Default|GetAlert%20Enemies) 1) 0 999)))))

(event EventResetMusicState
  (params (Music%20State :type Float%20%28single-precision%29))
  (Variables|Default|SetAlert%20Enemies 0)
  (Variables|Default|SetTarget%20State Music%20State)
  (Development|PrintString "Is this not getting Called?"))

(fn ConstructionScript)