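; Interactable clutter prop that the player can pick up into an inventory and throw to create noise.
; Interaction disables its physics and collision, then hands it to the interactor's InventoryComponent.
; Throwing adds a ProjectileMovement component at runtime with the given velocity.
; The first hit destroys that component, passes its velocity back to simulated physics, and reports a "Clutter"-tagged noise event at the impact point.
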(event OnComponentHit(StaticMesh)
  (params (HitComponent :type Primitive%20Component%20Object%20Reference) (OtherActor :type Actor%20Object%20Reference) (OtherComp :type Primitive%20Component%20Object%20Reference) (NormalImpulse :type Vector :default "0, 0, 0") (Hit :type Hit%20Result%20Structure%20%28by%20ref%29))
  (Utilities|IsValid (Variables|Default|GetProjectileMovement)
    (:Is%20Valid
      (CallFunction|DestroyProjectileMovement)
      (Class|AISenseHearing|ReportNoiseEvent (.Location (Collision|BreakHitResult Hit)) 0.5 self 0.0 "Clutter"))))

(event Custom|On%20Throw
  (params (ThrowVelocity :type Vector))
  (Utilities|IsValid (Variables|Default|GetProjectileMovement)
    (:Is%20Valid
      _)
    (:Is%20Not%20Valid
      (bind _returnvalue (AddComponent|AddProjectileMovementComponent))))
  (bind _output_get (Variables|Default|SetProjectileMovement _returnvalue))
  (Variables|/Script/Engine.MovementComponent|SetVelocity _output_get ThrowVelocity))

(event EventOnInteraction
  (params (Interactor :type Actor%20Object%20Reference))
  (bind _returnvalue (Actor|GetComponentbyClass Interactor "/Game/Blueprints/Player/Inventory/InventoryComponent.InventoryComponent_C"))
  (bind _staticmesh (Variables|Default|GetStaticMesh))
  (Utilities|IsValid _returnvalue
    (:Is%20Valid
      (Physics|SetSimulatePhysics _staticmesh false)
      (Collision|SetCollisionEnabled _staticmesh "NoCollision")
      (Default|PickupClutterObject _returnvalue self))))

(fn ConstructionScript)

(fn GetWidgetText
  (return "Pick Up"))

(fn GetInteractionAttach
  (return (Variables|Default|GetStaticMesh)))

(fn DestroyProjectileMovement
  (bind _staticmesh (Variables|Default|GetStaticMesh))
  (bind _projectilemovement (Variables|Default|GetProjectileMovement))
  (if (Utilities|IsValid _projectilemovement)
    (LocalVariables|SetLocalVelocity (Variables|/Script/Engine.MovementComponent|GetVelocity _projectilemovement))
    (Components|DestroyComponent (Variables|Default|GetProjectileMovement))
    (Physics|SetSimulatePhysics _staticmesh true)
    (Physics|SetPhysicsLinearVelocity _staticmesh (LocalVariables|GetLocalVelocity) false "None")))