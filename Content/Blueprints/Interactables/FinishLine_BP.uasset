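; FinishLine_BP is an interactable finish point that shows the prompt "Upload Worm" and ends the game in a win when used.
; It supplies the interaction prompt text and the WidgetAttach component as its attach point.
; On interaction, it unpossesses player controller 0, adds a You_Win_Screen widget to the viewport and shows the mouse cursor.
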(event EventBeginPlay)

(event Collision|EventActorBeginOverlap
  (params (OtherActor :type Actor%20Object%20Reference)))

(event EventTick
  (params (DeltaSeconds :type Float%20%28single-precision%29)))

(event EventOnInteraction
  (params (Interactor :type Actor%20Object%20Reference))
  (Pawn|UnPossess (Game|GetPlayerController 0))
  (bind _returnvalue (UserInterface|CreateWidget "/Game/UI/You_Win_Screen.You_Win_Screen_C"))
  (UserInterface|Viewport|AddtoViewport _returnvalue 0)
  (Variables|/Script/Engine.PlayerController|SetbShowMouseCursor (Game|GetPlayerController 0) true))

(fn ConstructionScript
  (|CallParentFunction))

(fn GetInteractionAttach
  (return (Variables|Default|GetWidget%20Attach)))

(fn GetWidgetText
  (return "Upload Worm"))