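; Base-style interactable Blueprint that shows a screen-space prompt while an interactor is in range and prints a debug string on interaction.
; Entering range creates an InteractPrompt_Widget for the interactor's player controller inside a runtime-added WidgetComponent, snapped to GetInteractionAttach; exiting range destroys it.
; GetWidgetText supplies a default label, while GetInteractionAttach returns no component here.
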(event EventOnInteractionRangeEntered
  (params (Interactor :type ALS%20Player%20Character%20BP%20Object%20Reference))
  (Variables|Default|GetInteractPrompt%20Widget
    (:then)
    (:else
      (bind _returnvalue (UserInterface|CreateWidget "/Game/UI/InteractPrompt_Widget.InteractPrompt_Widget_C" (.AsPlayer%20Controller (Utilities|Casting|CastToPlayerController (Pawn|GetController Interactor))) (Private|GetWidgetText)))
      (bind _returnvalue_2 (AddComponent|AddWidgetComponent false (Math|Transform|MakeTransform (Variables|Default|GetWidgetOffset) "0, 0, 0" "1,1,1")))
      (bind _output_get (Variables|Default|SetInteractPrompt%20Widget _returnvalue_2))
      (UserInterface|SetWidget _output_get _returnvalue)
      (Class|WidgetComponent|SetWidgetSpace _output_get "Screen")
      (Class|WidgetComponent|SetDrawatDesiredSize _output_get true)
      (Collision|SetCollisionEnabled _output_get "NoCollision")
      (Transformation|AttachComponentToComponent _output_get (Private|GetInteractionAttach) "None" "SnapToTarget" "SnapToTarget" "SnapToTarget" true))))

(event EventOnInteractionRangeExited
  (params (Interactor :type ALS%20Player%20Character%20BP%20Object%20Reference))
  (bind _interactprompt_widget (Variables|Default|GetInteractPrompt%20Widget)
    (:then
      (Components|DestroyComponent _interactprompt_widget))
    (:else)))

(event EventOnInteraction
  (params (Interactor :type ALS%20Player%20Character%20BP%20Object%20Reference))
  (Development|PrintString "Interacted"))

(fn ConstructionScript)

(fn GetInteractionAttach
  (return 0))

(fn GetWidgetText
  (return "Interact"))