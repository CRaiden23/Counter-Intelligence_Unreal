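; Ammo pickup interactable that gives an interacting actor a quantity of primary or secondary ammo.
; On BeginPlay it sets its static mesh by ammo type, though both types currently use the same AmmoBox mesh.
; Interaction prints a debug string, then adds the ammo to the interactor's InventoryComponent and destroys the pickup if that component exists.
; It also supplies the mesh as the interaction attach point and type-based prompt text.
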(event EventOnInteraction
  (params (Interactor :type ALS%20Player%20Character%20BP%20Object%20Reference))
  (bind _returnvalue (Actor|GetComponentbyClass Interactor "/Game/Blueprints/Player/Inventory/InventoryComponent.InventoryComponent_C"))
  (Development|PrintString (Utilities|String|Append (Utilities|String|EnumtoString (Variables|Default|GetPickupType)) " " (Utilities|String|ToString(Integer) (Variables|Default|GetQuantity))))
  (Utilities|IsValid _returnvalue
    (:Is%20Valid
      (Default|AddEquipment _returnvalue (Variables|Default|GetPickupType) (Variables|Default|GetQuantity))
      (Actor|DestroyActor))))

(event EventBeginPlay
  (bind _staticmesh (Variables|Default|GetStaticMesh))
  ;[1 1 1] Change Mesh Based on Ammo Type
  (switch Utilities|FlowControl|Switch|SwitchonE_PickupType (Variables|Default|GetPickupType)
    (:NewEnumerator0
      (Components|StaticMesh|SetStaticMesh _staticmesh "/Game/PlaceHolderMesh/AmmoBox.AmmoBox"))
    (:NewEnumerator1
      (Components|StaticMesh|SetStaticMesh _staticmesh "/Game/PlaceHolderMesh/AmmoBox.AmmoBox"))))

(fn ConstructionScript
  (|CallParentFunction))

(fn GetInteractionAttach
  (return (Variables|Default|GetStaticMesh)))

(fn GetWidgetText
  (return (Utilities|Text|ToText(String) (Utilities|String|Append "Pickup " (Utilities|String|EnumtoString (Variables|Default|GetPickupType)) " Ammo"))))