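; Grenade pickup interactable that grants grenades to any interactor with an InventoryComponent.
; On interaction it adds the quantity as equipment, passes the grenade class to the inventory and plays a pitch-randomized sound.
; It then either hides and disables collision for a short respawn delay or destroys itself.
; Its widget text joins the first two underscore-separated parts of the grenade class name.
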(event EventOnInteraction
  (params (Interactor :type Actor%20Object%20Reference))
  (bind _returnvalue (Actor|GetComponentbyClass Interactor "/Game/Blueprints/Player/Inventory/InventoryComponent.InventoryComponent_C"))
  (Utilities|IsValid _returnvalue
    (:Is%20Valid
      (Default|AddEquipment _returnvalue "NewEnumerator2" (Variables|Default|GetQuantity))
      (Default|PickupNewGrenade _returnvalue (Variables|Default|GetGrenade%20Class))
      (Audio|PlaySoundatLocation "/Game/Sounds/Pistol02/Pistol_Holster.Pistol_Holster" (Transformation|GetActorLocation) "0, 0, 0" 0.5 (Math|Random|RandomFloatinRange 0.75 1.25) 0.0 0 0 0)
      (if (Variables|Default|GetRespawn?)
        (Collision|SetActorEnableCollision false)
        (Rendering|SetActorHiddenInGame true)
        (Utilities|FlowControl|Delay 3.0)
        (Collision|SetActorEnableCollision true)
        (Rendering|SetActorHiddenInGame false)
        (else
          (Actor|DestroyActor))))))

(fn ConstructionScript
  (|CallParentFunction))

(fn GetWidgetText
  (bind _grenade_class (Variables|Default|GetGrenade%20Class))
  (bind _returnvalue (Utilities|GetClassDisplayName _grenade_class))
  (bind (_lefts _rights) (Utilities|String|Split _returnvalue "_"))
  (return (Utilities|Text|ToText(String) (Utilities|String|Append _lefts " " (.LeftS (Utilities|String|Split _rights "_"))))))