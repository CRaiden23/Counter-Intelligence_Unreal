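; Key pickup interactable that adds a named key item to the interacting actor's inventory.
; On interaction, it passes KeyItemName to the interactor's InventoryComponent, plays a randomly pitched pickup sound and destroys itself, doing nothing if that component is missing.
; Widget text comes from KeyItemName split at an underscore, with both halves rejoined without it.
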(event EventBeginPlay)

(event Collision|EventActorBeginOverlap
  (params (OtherActor :type Actor%20Object%20Reference)))

(event EventTick
  (params (DeltaSeconds :type Float%20%28single-precision%29)))

(event EventOnInteraction
  (params (Interactor :type Actor%20Object%20Reference))
  (bind _returnvalue (Actor|GetComponentbyClass Interactor "/Game/Blueprints/Player/Inventory/InventoryComponent.InventoryComponent_C"))
  ;[1 1 1] Add to player Inventory
  (Utilities|IsValid _returnvalue
    (:Is%20Valid
      (Default|PickupKeyItem _returnvalue (Variables|Default|GetKeyItemName))
      (Audio|PlaySoundatLocation "/Game/Sounds/Pistol02/Pistol_Holster_02.Pistol_Holster_02" (Transformation|GetActorLocation) "0, 0, 0" 0.5 (Math|Random|RandomFloatinRange 0.75 1.25) 0.0 0 0 0)
      (Actor|DestroyActor))))

(fn ConstructionScript
  (|CallParentFunction))

(fn GetWidgetText
  (bind _keyitemname (Variables|Default|GetKeyItemName))
  (bind (_lefts _rights) (Utilities|String|Split _keyitemname "_"))
  (return (Utilities|Text|ToText(String) (Utilities|String|Append _lefts " " _rights))))