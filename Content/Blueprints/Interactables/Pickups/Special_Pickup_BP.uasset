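; Interactable pickup that grants a quantity of a Special equipment item to the interactor's inventory component.
; If no Special is set, it picks a random one on BeginPlay, and its widget text shows the enum name.
; On pickup it plays a pitch-varied sound, then either hides and disables collision for a short delay before reappearing, or destroys itself, depending on the Respawn flag.
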(event EventBeginPlay
  (switch Utilities|FlowControl|Switch|SwitchonSpecials (Variables|Default|GetSpecial)
    (:NewEnumerator5
      (Variables|Default|SetSpecial (Utilities|Enum|ByteToEnumSpecials (Math|Conversions|ToByte(Integer) (Math|Random|RandomIntegerinRange 1 5)))))))

(event EventOnInteraction
  (params (Interactor :type Actor%20Object%20Reference))
  (bind _returnvalue (Actor|GetComponentbyClass Interactor "/Game/Blueprints/Player/Inventory/InventoryComponent.InventoryComponent_C"))
  (Utilities|IsValid _returnvalue
    (:Is%20Valid
      (Default|PickupNewEquipment _returnvalue (Variables|Default|GetSpecial) (Variables|Default|GetQuantity))
      (Audio|PlaySoundatLocation "/Game/Sounds/Pistol02/Pistol_Holster.Pistol_Holster" (Transformation|GetActorLocation) "0, 0, 0" 0.5 (Math|Random|RandomFloatinRange 0.75 1.25) 0.0 0 0 0)
      (if (Variables|Default|GetRespawn?)
        (Collision|SetActorEnableCollision false)
        (Rendering|SetActorHiddenInGame true)
        (Utilities|FlowControl|Delay 3.0)
        (Collision|SetActorEnableCollision true)
        (Rendering|SetActorHiddenInGame false)
        (else
          (Actor|DestroyActor))))))

(fn ConstructionScript
  (|CallParentFunction))

(fn GetWidgetText
  (return (Utilities|Text|ToText(String) (Utilities|String|EnumtoString (Variables|Default|GetSpecial)))))