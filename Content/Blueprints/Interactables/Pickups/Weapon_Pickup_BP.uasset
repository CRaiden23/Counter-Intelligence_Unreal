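; Interactable weapon pickup that gives its configured weapon class to whoever interacts with it.
; On interaction it finds the interactor's InventoryComponent, passes it the weapon class and pickup type, plays a holster sound with randomized pitch, then destroys itself.
; Interaction prompts attach to the static mesh, with label text derived from the weapon class display name before the first underscore.
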(event EventTick
  (params (DeltaSeconds :type Float%20%28single-precision%29)))

(event EventOnInteraction
  (params (Interactor :type ALS%20Player%20Character%20BP%20Object%20Reference))
  (bind _returnvalue (Actor|GetComponentbyClass Interactor "/Game/Blueprints/Player/Inventory/InventoryComponent.InventoryComponent_C"))
  (Utilities|IsValid _returnvalue
    (:Is%20Valid
      (Default|PickupNewWeapon _returnvalue (Variables|Default|GetWeaponClass) (Variables|Default|GetPickupType))
      (Audio|PlaySoundatLocation "/Game/Sounds/Assault_Rifle02/AR_Holster.AR_Holster" (Transformation|GetActorLocation) "0, 0, 0" 0.5 (Math|Random|RandomFloatinRange 0.75 1.25) 0.0 0 0 0)
      (Actor|DestroyActor))))

(event EventBeginPlay)

(fn ConstructionScript
  (|CallParentFunction))

(fn GetInteractionAttach
  (return (Variables|Default|GetStaticMesh)))

(fn GetWidgetText
  (return (Utilities|Text|ToText(String) (.LeftS (Utilities|String|Split (Utilities|GetClassDisplayName (Variables|Default|GetWeaponClass)) "_")))))