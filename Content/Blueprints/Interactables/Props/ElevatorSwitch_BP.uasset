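; Interactable elevator call switch that opens the elevator doors and handles the streamed transition from Level0 to Level1.
; Interacting once shows a wait prompt, then marks arrival and opens the doors after a delay, suppressing further range prompts.
; When the ALS player overlaps the Box, timed steps close the doors, unload Level0, load Level1 with blocking, then reopen.
; Doors snap between positions through relative world-space teleports rather than animation.
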(event OnComponentBeginOverlap(Box)
  (params (OverlappedComponent :type Primitive%20Component%20Object%20Reference) (OtherActor :type Actor%20Object%20Reference) (OtherComp :type Primitive%20Component%20Object%20Reference) (OtherBodyIndex :type Integer) (bFromSweep :type Boolean) (SweepResult :type Hit%20Result%20Structure%20%28by%20ref%29))
  (Utilities|Casting|CastToALS_Player_CharacterBP OtherActor)
  (Utilities|FlowControl|Delay 1.0)
  (CallFunction|ResetDoorPosition)
  (Utilities|FlowControl|Delay 1.0)
  (Game|UnloadStreamLevel(byName) "Level0" false)
  (Game|LoadStreamLevel(byName) "Level1" true true)
  (Utilities|FlowControl|Delay 1.0)
  (CallFunction|OpenDoors))

(event EventOnInteractionRangeEntered
  (params (Interactor :type ALS%20Player%20Character%20BP%20Object%20Reference))
  (if (not (Variables|Default|GethasArrived))
    (|CallParentFunction Interactor)))

(event EventOnInteraction
  (params (Interactor :type ALS%20Player%20Character%20BP%20Object%20Reference))
  (if (not (Variables|Default|GethasArrived))
    (if (not (Variables|Default|GetisCalled))
      (Variables|Default|SetisCalled true)
      (Utilities|FlowControl|Delay 1.0)
      (Variables|Default|SethasArrived true)
      (CallFunction|OpenDoors))))

(fn ConstructionScript
  (|CallParentFunction))

(fn GetInteractionAttach
  (return (Variables|Default|GetStaticMesh)))

(fn ResetDoorPosition
  (Transformation|SetWorldLocation (Variables|Default|GetDoorL) (+ (Transformation|GetWorldLocation (Variables|Default|GetDoorL)) (Math|Vector|MakeVector 1.5e+02 0.0 0.0)) false true)
  (Transformation|SetWorldLocation (Variables|Default|GetDoorR) (+ (Transformation|GetWorldLocation (Variables|Default|GetDoorR)) (Math|Vector|MakeVector -1.5e+02 0.0 0.0)) false true))

(fn GetWidgetText
  (if (Variables|Default|GetisCalled)
    (return "Please Wait...")
    (else
      (return "Call"))))

(fn OpenDoors
  (Transformation|SetWorldLocation (Variables|Default|GetDoorL) (+ (Transformation|GetWorldLocation (Variables|Default|GetDoorL)) (Math|Vector|MakeVector -1.5e+02 0.0 0.0)) false true)
  (Transformation|SetWorldLocation (Variables|Default|GetDoorR) (+ (Transformation|GetWorldLocation (Variables|Default|GetDoorR)) (Math|Vector|MakeVector 1.5e+02 0.0 0.0) "") false true))