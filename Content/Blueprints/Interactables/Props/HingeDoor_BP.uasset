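; Interactable hinged door that opens, closes, and can start locked, with a prompt reflecting its state.
; A lockpick charge unlocks it quietly without opening, while forcing it opens it and reports a noise event.
; A timeline swings the mesh 90 degrees, dropping collision to query-only until past halfway, with pitch-randomized sounds.
; The "Pick Lock" prompt checks inventory Battery, whereas the interaction checks and spends EquipmentAmmo.
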(event Custom|OnOpen
  (bind _staticmesh (Variables|Default|GetStaticMesh))
  (bind (_direction _door_rotate) (Timeline|DoorRotate Play)
    (:Update
      (switch Utilities|FlowControl|Switch|SwitchonETimelineDirection _direction
        (:Forward
          (if (> _door_rotate 0.5)
            (Collision|SetCollisionEnabled _staticmesh "QueryAndPhysics" :!label _label)))
        (:Backward
          (if (< _door_rotate 0.5)
            (goto _label)
            (else
              _))))
      (Transformation|SetRelativeRotation _staticmesh (Math|Rotator|MakeRotator 0.0 0.0 (* _door_rotate 9e+01)) false false))
    (:Finished
      (if (not (Variables|Default|GetbIsOpen))
        (Audio|PlaySoundatLocation "/Game/Sounds/InteractableSounds/Door_Close_5.Door_Close_5" (Transformation|GetWorldLocation (Variables|Default|GetScene)) "0, 0, 0" 0.5 (+ (Math|Random|RandomFloatinRange -0.1 0.1) 1.0) 0.0 "/Game/Sounds/Sound_Falloff.Sound_Falloff" 0 0)))))

(event Custom|OnClose
  (bind _staticmesh (Variables|Default|GetStaticMesh))
  (bind (_direction _door_rotate) (Timeline|DoorRotate Reverse)
    (:Update
      (switch Utilities|FlowControl|Switch|SwitchonETimelineDirection _direction
        (:Forward
          (if (> _door_rotate 0.5)
            (Collision|SetCollisionEnabled _staticmesh "QueryAndPhysics" :!label _label)))
        (:Backward
          (if (< _door_rotate 0.5)
            (goto _label)
            (else
              _))))
      (Transformation|SetRelativeRotation _staticmesh (Math|Rotator|MakeRotator 0.0 0.0 (* _door_rotate 9e+01)) false false))
    (:Finished
      (if (not (Variables|Default|GetbIsOpen))
        (Audio|PlaySoundatLocation "/Game/Sounds/InteractableSounds/Door_Close_5.Door_Close_5" (Transformation|GetWorldLocation (Variables|Default|GetScene)) "0, 0, 0" 0.5 (+ (Math|Random|RandomFloatinRange -0.1 0.1) 1.0) 0.0 "/Game/Sounds/Sound_Falloff.Sound_Falloff" 0 0)))))

(event EventOnInteractionRangeEntered
  (params (Interactor :type ALS%20Player%20Character%20BP%20Object%20Reference))
  (Variables|Default|SetPlayerInv (Actor|GetComponentbyClass Interactor "/Game/Blueprints/Player/Inventory/InventoryComponent.InventoryComponent_C"))
  (|CallParentFunction Interactor))

(event EventOnInteraction
  (params (Interactor :type ALS%20Player%20Character%20BP%20Object%20Reference))
  (bind _returnvalue (Actor|GetComponentbyClass Interactor "/Game/Blueprints/Player/Inventory/InventoryComponent.InventoryComponent_C"))
  (bind _self self)
  (if (Variables|Default|GetbIsLocked)
    (Utilities|IsValid _returnvalue
      (:Is%20Valid
        ;[1 1 1] Do we have a lockpick?
        (bind _output_get (Variables|Default|SetPlayerInv _returnvalue))
        (if (and (Utilities|Enum|Equal(Enum) (Variables|/Game/Blueprints/Player/Inventory/InventoryComponent.InventoryComponent_C|GetSpecial _output_get) "NewEnumerator0") (> (Variables|/Game/Blueprints/Player/Inventory/InventoryComponent.InventoryComponent_C|GetEquipmentAmmo _output_get) 0))
          (Variables|Default|SetbIsLocked false)
          (CallFunction|OnInteractionRangeExited)
          (Variables|/Game/Blueprints/Player/Inventory/InventoryComponent.InventoryComponent_C|SetEquipmentAmmo (Variables|Default|GetPlayerInv) (- (Variables|/Game/Blueprints/Player/Inventory/InventoryComponent.InventoryComponent_C|GetEquipmentAmmo (Variables|Default|GetPlayerInv)) 1))
          (else
            (Variables|Default|SetbIsLocked false)
            (CallFunction|OpenDoor)
            (Class|AISenseHearing|ReportNoiseEvent (Transformation|GetActorLocation _self) 1.0 _self 5e+02 "Sound")))))
    (else
      (if (Variables|Default|GetbIsOpen)
        (CallFunction|CloseDoor)
        (else
          (CallFunction|OpenDoor)))
      (CallFunction|OnInteractionRangeExited))))

(fn ConstructionScript
  (|CallParentFunction))

(fn GetWidgetText
  (bind _playerinv (Variables|Default|GetPlayerInv))
  (if (Variables|Default|GetbIsLocked)
    (if (and (Utilities|Enum|Equal(Enum) (Variables|/Game/Blueprints/Player/Inventory/InventoryComponent.InventoryComponent_C|GetSpecial _playerinv) "NewEnumerator0") (> (Variables|/Game/Blueprints/Player/Inventory/InventoryComponent.InventoryComponent_C|GetBattery _playerinv) 0.0))
      (return "Pick Lock")
      (else
        (return "Force Open")))
    (elif (Variables|Default|GetbIsOpen)
      (return "Close")
      (else
        (return "Open")))))

(fn GetInteractionAttach
  (return (Variables|Default|GetWidget%20Attach)))

(fn CloseDoor
  (Variables|Default|SetbIsOpen false)
  (Collision|SetCollisionEnabled (Variables|Default|GetStaticMesh) "QueryOnly")
  (CallFunction|OnClose)
  (return))

(fn OpenDoor
  (Collision|SetCollisionEnabled (Variables|Default|GetStaticMesh) "QueryOnly")
  (Audio|PlaySoundatLocation "/Game/Sounds/InteractableSounds/Door_Open_3.Door_Open_3" (Transformation|GetWorldLocation (Variables|Default|GetScene)) "0, 0, 0" 0.5 (+ (Math|Random|RandomFloatinRange -0.1 0.1) 1.0) 0.0 "/Game/Sounds/Sound_Falloff.Sound_Falloff" 0 0)
  (Variables|Default|SetbIsOpen true)
  (CallFunction|OnOpen)
  (Variables|Default|SetbIsLocked false)
  (return))