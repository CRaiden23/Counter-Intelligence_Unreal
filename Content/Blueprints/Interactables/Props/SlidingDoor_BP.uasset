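; Interactable sliding door prop that toggles open and closed on interaction unless it is locked.
; Interacting offsets the static mesh's world location by a set distance along a selectable X, Y or Z axis, reversing the offset to close.
; The move is an instant teleport, marked to become a lerp later, followed by a call to OnInteractionRangeExited.
; The interaction widget reads Locked, Open or Close from the current state.
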(event EventOnInteraction
  (params (Interactor :type ALS%20Player%20Character%20BP%20Object%20Reference))
  (bind _staticmesh (Variables|Default|GetStaticMesh))
  (bind _staticmesh_2 (Variables|Default|GetStaticMesh))
  (bind _distancetotravel (Variables|Default|GetDistanceToTravel))
  (bind _distancetotravel_2 (Variables|Default|GetDistanceToTravel))
  (bind _returnvalue (Transformation|GetWorldLocation _staticmesh))
  (bind _returnvalue_2 (Transformation|GetWorldLocation _staticmesh_2))
  (if (Variables|Default|GetbIsLocked)
    (Development|PrintString "Locked")
    (else
      (if (Variables|Default|GetbIsOpen)
        (Variables|Default|SetbIsOpen false)
        (switch Utilities|FlowControl|Switch|SwitchonESplineMeshAxis (Variables|Default|GetSlidingAxis)
          (:X
            (Variables|Default|SetDestination (- _returnvalue_2 (Math|Vector|MakeVector _distancetotravel_2 0.0 0.0))))
          (:Y
            (Variables|Default|SetDestination (- _returnvalue_2 (Math|Vector|MakeVector 0.0 _distancetotravel_2 0.0))))
          (:Z
            (Variables|Default|SetDestination (- _returnvalue_2 (Math|Vector|MakeVector 0.0 0.0 _distancetotravel_2)))))
        (else
          (Variables|Default|SetbIsOpen true)
          (switch Utilities|FlowControl|Switch|SwitchonESplineMeshAxis (Variables|Default|GetSlidingAxis)
            (:X
              (Variables|Default|SetDestination (+ _returnvalue (Math|Vector|MakeVector _distancetotravel 0.0 0.0))))
            (:Y
              (Variables|Default|SetDestination (+ _returnvalue (Math|Vector|MakeVector 0.0 _distancetotravel 0.0))))
            (:Z
              (Variables|Default|SetDestination (+ _returnvalue (Math|Vector|MakeVector 0.0 0.0 _distancetotravel)))))))
      ;[1 1 1] CHANGE TO LERP LATER
      (Transformation|SetWorldLocation (Variables|Default|GetStaticMesh) (Variables|Default|GetDestination) false true)
      (CallFunction|OnInteractionRangeExited))))

(fn ConstructionScript)

(fn GetWidgetText
  (if (Variables|Default|GetbIsLocked)
    (return "Locked")
    (elif (Variables|Default|GetbIsOpen)
      (return "Close")
      (else
        (return "Open")))))

(fn GetInteractionAttach
  (return (Variables|Default|GetScene)))