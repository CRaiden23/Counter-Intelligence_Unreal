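; Interactable tutorial exit door that the player calls, then enters to end the level and return to the main menu.
; Interaction shows a "Please Wait..." prompt during a short delay, then slides both doors apart by timeline along a selectable axis and enables the trigger box.
; The first player overlap closes the doors after a delay, fades to black through a widget and loads Main_Menu.
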(event OnComponentBeginOverlap(Box)
  (params (OverlappedComponent :type Primitive%20Component%20Object%20Reference) (OtherActor :type Actor%20Object%20Reference) (OtherComp :type Primitive%20Component%20Object%20Reference) (OtherBodyIndex :type Integer) (bFromSweep :type Boolean) (SweepResult :type Hit%20Result%20Structure%20%28by%20ref%29))
  (Utilities|Casting|CastToALS_Player_CharacterBP OtherActor)
  (Utilities|FlowControl|DoOnce false
    (:Completed
      (Utilities|FlowControl|Delay 1.5)
      (CallFunction|SlideDoors false)
      (bind _returnvalue (UserInterface|CreateWidget "/Game/UI/FadeToBlack.FadeToBlack_C"))
      (bind _output_get (Variables|Default|SetFadeToBlack _returnvalue))
      (UserInterface|Viewport|AddtoViewport _output_get 0)
      (Class|UserWidget|PlayAnimationForward (Variables|Default|GetFadeToBlack) (Variables|/Game/UI/FadeToBlack.FadeToBlack_C|GetFade (Variables|Default|GetFadeToBlack)) 1.0 false)
      (Utilities|FlowControl|Delay 2.75)
      (Game|OpenLevel(byObjectReference) "/Game/Levels/Menus/Main_Menu.Main_Menu"))))

(event Custom|Slide%20Doors
  (params (Open%20Door :type Boolean))
  (if Open%20Door
    (bind _door_slide (Timeline|Door%20Slide Play)
      (:Update
        (switch Utilities|FlowControl|Switch|SwitchonESplineMeshAxis (Variables|Default|GetSliding%20Axis)
          (:X
            (Transformation|SetRelativeLocation (Variables|Default|GetDoorL) (Math|Vector|MakeVector (* _door_slide -75.0) 0.0 0.0) false false)
            (Transformation|SetRelativeLocation (Variables|Default|GetDoorR) (Math|Vector|MakeVector (* _door_slide 75.0) 0.0 0.0) false false))
          (:Y
            (Transformation|SetRelativeLocation (Variables|Default|GetDoorL) (Math|Vector|MakeVector 0.0 (* _door_slide -75.0) 0.0) false false)
            (Transformation|SetRelativeLocation (Variables|Default|GetDoorR) (Math|Vector|MakeVector 0.0 (* _door_slide 75.0) 0.0) false false))
          (:Z
            (Transformation|SetRelativeLocation (Variables|Default|GetDoorL) (Math|Vector|MakeVector 0.0 0.0 (* _door_slide -75.0)) false false)
            (Transformation|SetRelativeLocation (Variables|Default|GetDoorR) (Math|Vector|MakeVector 0.0 0.0 (* _door_slide 75.0)) false false)))))
    (else
      (Timeline|Door%20Slide Reverse))))

(event EventOnInteractionRangeEntered
  (params (Interactor :type ALS%20Player%20Character%20BP%20Object%20Reference))
  (if (not (Variables|Default|GethasArrived))
    (|CallParentFunction Interactor)))

(event EventOnInteraction
  (params (Interactor :type Actor%20Object%20Reference))
  (if (not (Variables|Default|GethasArrived))
    (if (not (Variables|Default|GetisCalled))
      (Variables|Default|SetisCalled true)
      (Utilities|FlowControl|Delay 2.5)
      (Variables|Default|SethasArrived true)
      (CallFunction|SlideDoors true)
      (Collision|SetCollisionEnabled (Variables|Default|GetBox) "QueryAndPhysics"))))

(fn ConstructionScript
  (|CallParentFunction))

(fn GetInteractionAttach
  (return (Variables|Default|GetStaticMesh)))

(fn ResetDoorPosition
  (Transformation|SetWorldLocation (Variables|Default|GetDoorL) (+ (Transformation|GetWorldLocation (Variables|Default|GetDoorL)) (Math|Vector|MakeVector 1.5e+02 0.0 0.0)) false true)
  (Transformation|SetWorldLocation (Variables|Default|GetDoorR) (+ (Transformation|GetWorldLocation (Variables|Default|GetDoorR)) (Math|Vector|MakeVector -1.5e+02 0.0 0.0)) false true))

(fn GetWidgetText
  (if (Variables|Default|GetisCalled)
    (return "Please Wait...")
    (else
      (return "Call"))))