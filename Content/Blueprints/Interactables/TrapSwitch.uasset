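; TrapSwitch is an interactable switch that toggles the traps in its Traps array.
; On interaction it waits briefly, flips IsActive, then calls Activate or Deactivate on each trap; the prompt text follows IsActive.
; A Delay inside the activation loop later runs the shared deactivation loop, shutting traps off automatically.
; That timed shutoff bypasses the IsActive reset, so the prompt still reads "Deactivate".
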(event EventBeginPlay)

(event Collision|EventActorBeginOverlap
  (params (OtherActor :type Actor%20Object%20Reference)))

(event EventTick
  (params (DeltaSeconds :type Float%20%28single-precision%29)))

(event EventOnInteraction
  (params (Interactor :type Actor%20Object%20Reference))
  (if (Variables|Default|GetisActive)
    (Utilities|FlowControl|Delay 1.0)
    (Variables|Default|SetisActive false)
    (for _array_element (Variables|Default|GetTraps) :!label _label
      (Default|Deactivate _array_element))
    (else
      (Utilities|FlowControl|Delay 1.0)
      (Variables|Default|SetisActive true)
      (for _array_element_2 (Variables|Default|GetTraps)
        (Default|Activate _array_element_2)
        (Utilities|FlowControl|Delay 5.0)
        (goto _label)))))

(fn ConstructionScript
  (|CallParentFunction))

(fn GetWidgetText
  (return (select (Variables|Default|GetisActive) "Deactivate" "Activate")))

(fn GetInteractionAttach
  (return (Variables|Default|GetWidgetAttach)))