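; Frag grenade actor that explodes on a timed fuse, dealing full, non-falloff radial damage.
; BeginPlay starts the Explode timer and sets TimerSet; mesh hits share that path but only arm it if the flag is unset.
; Explode applies damage, reports an AI noise event, draws a debug sphere of the radius, spawns Explosion_BP and destroys the grenade.
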(event OnComponentHit(StaticMesh)
  (params (HitComponent :type Primitive%20Component%20Object%20Reference) (OtherActor :type Actor%20Object%20Reference) (OtherComp :type Primitive%20Component%20Object%20Reference) (NormalImpulse :type Vector :default "0, 0, 0") (Hit :type Hit%20Result%20Structure%20%28by%20ref%29))
  (if (.bBlockingHit (Collision|BreakHitResult Hit))
    (if (not (Variables|Default|GetTimer%20Set))
      (Variables|Default|SetTimer%20Set true)
      (Utilities|Time|SetTimerbyFunctionName 0 "Explode" (Variables|Default|GetTimer%20Length)))))

(event EventBeginPlay
  (|CallParentFunction)
  (Variables|Default|SetTimer%20Set true)
  (Utilities|Time|SetTimerbyFunctionName 0 "Explode" (Variables|Default|GetTimer%20Length)))

(fn ConstructionScript
  (|CallParentFunction))

(fn Explode
  (bind _staticmesh (Variables|Default|GetStaticMesh))
  (bind _effective_radius (Variables|Default|GetEffective%20Radius))
  (bind _returnvalue (Transformation|GetWorldLocation _staticmesh))
  (Game|Damage|ApplyRadialDamage (Variables|Default|GetDamage) _returnvalue _effective_radius "/Script/Engine.DamageType" 0 0 0 true "ECC_Visibility")
  (Class|AISenseHearing|ReportNoiseEvent _returnvalue 2.0 self 6e+02 "Clutter")
  (Rendering|Debug|DrawDebugSphere _returnvalue _effective_radius 12 "(R=1.000000,G=0.272000,B=0.000000,A=1.000000)" 1.0)
  (Game|SpawnActorfromClass "/Game/Blueprints/Weapons/Explosion_BP.Explosion_BP_C" (Transformation|GetActorTransform) "AlwaysSpawn" 0 0)
  (Actor|DestroyActor))