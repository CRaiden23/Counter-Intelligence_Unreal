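; Frag grenade Blueprint, a timed explosive that extends a parent class and starts its fuse timer on BeginPlay.
; Explode applies full radial damage within its effective radius, reports a noise event, spawns Explosion_BP and hides the actor.
; It then sets a longer timer, and a separate Destroy function removes the actor.
; The component hit event is empty, and debug prints mark each stage.
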(event OnComponentHit(StaticMesh)
  (params (HitComponent :type Primitive%20Component%20Object%20Reference) (OtherActor :type Actor%20Object%20Reference) (OtherComp :type Primitive%20Component%20Object%20Reference) (NormalImpulse :type Vector :default "0, 0, 0") (Hit :type Hit%20Result%20Structure%20%28by%20ref%29)))

(event EventBeginPlay
  (|CallParentFunction)
  (Variables|Default|SetTimer%20Set true)
  (Development|PrintString "Timer Set")
  (Utilities|Time|SetTimerbyEvent (EventDispatchers|CreateEvent :!event Explode) (Variables|Default|GetTimer%20Length)))

(fn ConstructionScript
  (|CallParentFunction))

(fn Explode
  (bind _staticmesh (Variables|Default|GetStaticMesh))
  (bind _returnvalue (Transformation|GetWorldLocation _staticmesh))
  (Development|PrintString "BOOM!")
  (Game|Damage|ApplyRadialDamage (Variables|Default|GetDamage) _returnvalue (Variables|Default|GetEffective%20Radius) "/Script/Engine.DamageType" 0 0 0 true "ECC_Visibility")
  (Class|AISenseHearing|ReportNoiseEvent _returnvalue 2.0 self 1e+03 "Sound")
  (Game|SpawnActorfromClass "/Game/Blueprints/Weapons/Explosion_BP.Explosion_BP_C" (Transformation|GetActorTransform) "AlwaysSpawn" 0 0)
  (Rendering|SetActorHiddenInGame true)
  (Utilities|Time|SetTimerbyEvent (EventDispatchers|CreateEvent :!event Destroy) 25.0))

(fn Destroy
  (Development|PrintString "Destroyed")
  (Actor|DestroyActor))