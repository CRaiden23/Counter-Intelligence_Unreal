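; Ithaca 37 shotgun Blueprint that extends a parent weapon class with shell-by-shell reloading and its own fire behavior.
; Reload loops through a short Delay, adding one round with a mag-in sound each pass until the gun is full or the supplied ammo count is loaded.
; PrimaryFire is blocked while reloading, otherwise playing a cock sound before calling the parent; a note flags it as faulty for guards.
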(event EventReload
  (params (AmmoIn :type Integer))
  (Variables|Default|SetIsReloading true)
  (Variables|Default|SetReloading (+ (Variables|Default|GetReloading) 1) :!label _label)
  (Audio|PlaySoundatLocation (Utilities|Struct|BreakWeaponFX_Struct (Variables|Default|GetWeapon_FX)) (Transformation|GetWorldLocation (Variables|Default|GetWeaponMesh)) "0, 0, 0" 1.0 1.0 0.0 0 0 0)
  (bind _output_get (Variables|Default|SetCurrentAmmo (+ (Variables|Default|GetCurrentAmmo) 1)))
  (Utilities|FlowControl|Delay 0.3)
  (if (or (== _output_get (Variables|Default|GetMaxAmmo)) (== (Variables|Default|GetReloading) AmmoIn))
    (Variables|Default|SetReloading 0)
    (Variables|Default|SetIsReloading false)
    (else
      (goto _label))))

(event EventPrimaryFire
  ;[1 1 1] Doesn't Work Right for guards
  (if (not (Variables|Default|GetIsReloading))
    (Audio|PlaySoundatLocation (Utilities|Struct|BreakWeaponFX_Struct (Variables|Default|GetWeapon_FX)) (Transformation|GetWorldLocation (Variables|Default|GetWeaponMesh)) "0, 0, 0" 1.0 1.0 0.0 0 0 0)
    (|CallParentFunction)))

(fn ConstructionScript
  (|CallParentFunction))