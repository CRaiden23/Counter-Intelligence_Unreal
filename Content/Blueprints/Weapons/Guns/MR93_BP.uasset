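; MR93 gun Blueprint, a child weapon that defines its own round-by-round reload.
; Reload spawns one Niagara ejection effect per incoming round at the BulletEject point and plays the mag-out sound.
; A delay-driven loop then adds one round at a time with a mag-in sound, holding IsReloading until CurrentAmmo reaches MaxAmmo or all incoming rounds are loaded.
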(event EventBeginPlay)

(event EventReload
  (params (AmmoIn :type Integer))
  (bind _bullet_eject (Variables|Default|GetBullet%20Eject))
  (bind _weapon_fx (Variables|Default|GetWeapon_FX))
  (bind (_magout _magin) (Utilities|Struct|BreakWeaponFX_Struct _weapon_fx))
  (for _index (range 1 AmmoIn)
    (Niagara|SpawnSystematLocation "/Game/Gun_VFX/Niagara_FX/Bullet_ejection/NS_Pistol_Ejection_Effect.NS_Pistol_Ejection_Effect" (Transformation|GetWorldLocation _bullet_eject) (Transformation|GetWorldRotation _bullet_eject)))
  (Audio|PlaySoundatLocation _magout (Transformation|GetWorldLocation (Variables|Default|GetWeaponMesh)) "0, 0, 0" 1.0 1.0 0.0 0 0 0)
  (Utilities|FlowControl|Delay 0.2)
  (Variables|Default|SetIsReloading true)
  (Variables|Default|SetReloading (+ (Variables|Default|GetReloading) 1) :!label _label)
  (Audio|PlaySoundatLocation _magin (Transformation|GetWorldLocation (Variables|Default|GetWeaponMesh)) "0, 0, 0" 1.0 1.0 0.0 0 0 0)
  (bind _output_get (Variables|Default|SetCurrentAmmo (+ (Variables|Default|GetCurrentAmmo) 1)))
  (Utilities|FlowControl|Delay 0.3)
  (if (or (== _output_get (Variables|Default|GetMaxAmmo)) (== (Variables|Default|GetReloading) AmmoIn))
    (Variables|Default|SetReloading 0)
    (Variables|Default|SetIsReloading false)
    (else
      (goto _label))))

(event EventTick
  (params (DeltaSeconds :type Float%20%28single-precision%29)))

(event Collision|EventActorBeginOverlap
  (params (OtherActor :type Actor%20Object%20Reference)))

(fn ConstructionScript
  (|CallParentFunction))