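; Director actor that lets Twitch chat vote on events that disrupt the player, from guard alerts and spawns to lights out and locked doors.
; After TwitchIRC authenticates, timers cycle voting rounds, each announcing up to three random, distinct picks from the event enum.
; Numeric chat messages fill vote buckets, one vote per user.
; At round end the winner is announced and dispatched through an enum switch to guards, spawners, doors, post-process or player.
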(event OnMessageReceived(TwitchIRC)
  (params (Message :type String) (User :type String))
  (bind _returnvalue (Math|Conversions|ToInteger(Byte) Message))
  (bind _vote_buckets (Variables|VotingSystem|GetVote%20Buckets))
  (bind _returnvalue_2 (- _returnvalue 1))
  (if (Variables|VotingSystem|GetListening%20For%20Votes)
    ;[1 1 1] Ignore Users Who Already Voted
    (if (not (Utilities|Set|Contains (Variables|VotingSystem|GetVoters) User))
      (if (and (> _returnvalue 0) (<= _returnvalue (Utilities|Array|Length (Variables|VotingSystem|GetVote%20Buckets))))
        (Utilities|Array|SetArrayElem _vote_buckets _returnvalue_2 (+ (Utilities|Array|Get(acopy) _vote_buckets _returnvalue_2) 1))
        (Utilities|Set|Add (Variables|VotingSystem|GetVoters) User)))))

(event OnAuthentication(TwitchIRC)
  (bind _returnvalue (Utilities|Time|SetTimerbyEvent (delegate Custom|Begin%20Listening%20for%20Votes) 15.0 false 5.0 5.0))
  (Variables|Default|SetInit%20Votes%20Handle _returnvalue))

(event Custom|Begin%20Listening%20for%20Votes
  (bind _events_set (VotingSystem|SelectEventstoVoteon))
  (if _events_set
    (VotingSystem|AnnounceVoting)
    ;[1 1 1] Screen effect or sound event?
    (Development|PrintString "Listening for Votes!" false true "(R=1.000000,G=0.000000,B=0.258183,A=1.000000)" 5.0)
    (Variables|VotingSystem|SetListening%20For%20Votes true)
    (bind _returnvalue (Utilities|Time|SetTimerbyEvent (delegate Custom|Stop%20Listening%20for%20Votes) 3e+01))
    (Variables|Default|SetEnd%20Votes%20Handle _returnvalue)
    (else
      (Variables|VotingSystem|SetListening%20For%20Votes false))))

(event Custom|Stop%20Listening%20for%20Votes
  (bind _twitchirc (Variables|Default|GetTwitchIRC))
  (Utilities|FlowControl|Sequence
    (:then_0
      ;[1 1 1] Stop Listening, Set Winner
      (Development|PrintString "Voting Ended!" false true "(R=1.000000,G=0.000000,B=0.259243,A=1.000000)" 5.0)
      (bind _winning_event (VotingSystem|GetWinningEvent))
      (bind _output_get (Variables|VotingSystem|SetWinning%20Event _winning_event))
      (Variables|VotingSystem|SetListening%20For%20Votes false)
      (Utilities|Array|Clear (Variables|VotingSystem|GetVote%20Buckets))
      (Utilities|Array|Clear (Variables|VotingSystem|GetEvents%20To%20Be%20Voted%20On))
      (Utilities|Set|Clear (Variables|VotingSystem|GetVoters))
      (Class|TwitchIRCComponent|SendtoChat _twitchirc (Utilities|String|Append "Voting has ended! " (Utilities|String|Append "\"" (Utilities|String|EnumtoString _output_get) "\" Wins!")) (Variables|/Script/Counter_Intelligence.TwitchIRCComponent|GetChannelName _twitchirc)))
    (:then_1
      ;[1 1 1] Execute Winning Event
      (DirectorEvents|ExecuteDirectorEvent)
      (bind _returnvalue (Utilities|Time|SetTimerbyEvent (delegate Custom|Begin%20Listening%20for%20Votes) 10.5 false 15.0 1e+01))
      (Variables|Default|SetBegin%20Votes%20Handle _returnvalue))))

(event EventBeginPlay
  (Variables|Default|SetPlayerCharacter (Game|GetPlayerCharacter 0)))

(event EventDestroyed
  (CallFunction|ClearAllTimers))

(fn ConstructionScript)

(fn AnnounceVoting
  (bind _twitchirc (Variables|Default|GetTwitchIRC))
  (bind _twitchirc_2 (Variables|Default|GetTwitchIRC))
  (Class|TwitchIRCComponent|SendtoChat _twitchirc_2 "Voting has begun!" (Variables|/Script/Counter_Intelligence.TwitchIRCComponent|GetChannelName _twitchirc_2))
  (for (_array_element _array_index) (Variables|VotingSystem|GetEvents%20To%20Be%20Voted%20On)
    (Class|TwitchIRCComponent|SendtoChat _twitchirc (Utilities|String|Append (Utilities|String|ToString(Integer) (+ _array_index 1)) ": " (Utilities|String|EnumtoString _array_element) " 
") (Variables|/Script/Counter_Intelligence.TwitchIRCComponent|GetChannelName _twitchirc))))

(fn SelectEventstoVoteon
  (bind _numberofevents (LocalVariables|GetNumberOfEvents))
  (bind _returnvalue (Math|Conversions|ToInteger(Byte) _numberofevents))
  (bind _returnvalue_2 (- _returnvalue 1))
  ;[1 1 1] Fail Out If We Have Nothing To Vote For
  (if (!= _returnvalue 0)
    (for _index (range 0 (Math|Integer|Clamp(Integer) 2 0 _returnvalue_2))
      (bind _output_get (LocalVariables|SetRandIndex (Math|Random|RandomIntegerinRange 0 _returnvalue_2)))
      ;[1 1 1] Increment Random Number if we have already used it
      (while (Utilities|Set|Contains (LocalVariables|GetIndicesUsed) _output_get)
        (LocalVariables|SetRandIndex (Math|Integer|%(Integer) (+ (LocalVariables|GetRandIndex) 1) (Math|Conversions|ToInteger(Byte) (LocalVariables|GetNumberOfEvents)))))
      ;[1 1 1] Mark Index as used
      (Utilities|Set|Add (LocalVariables|GetIndicesUsed) (LocalVariables|GetRandIndex))
      ;[1 1 1] Add Event to our Voting Array
      (Utilities|Array|Add (Variables|VotingSystem|GetEvents%20To%20Be%20Voted%20On) (Utilities|Enum|ByteToEnumDirectorEvents_Enum (Math|Conversions|ToByte(Integer) (LocalVariables|GetRandIndex)))))
    ;[1 1 1] Resize Vote Buckets Appropriately
    (Utilities|Array|Resize (Variables|VotingSystem|GetVote%20Buckets) (Utilities|Array|Length (Variables|VotingSystem|GetEvents%20To%20Be%20Voted%20On)))
    (return true)
    (else
      (return false))))

(fn GetWinningEvent
  ;[1 1 1] Find the Winning Index
  (for (_array_element _array_index) (Variables|VotingSystem|GetVote%20Buckets)
    (if (> _array_element (LocalVariables|GetMax%20Votes))
      (LocalVariables|SetMax%20Votes _array_element)
      (LocalVariables|SetWinning%20Index _array_index)))
  (if (== (LocalVariables|GetWinning%20Index) -1)
    ;[1 1 1] 3-Way Tie
    (return (Utilities|Array|Get(acopy) (Variables|VotingSystem|GetEvents%20To%20Be%20Voted%20On) (Math|Random|RandomIntegerinRange 0 (- (Utilities|Array|Length (Variables|VotingSystem|GetEvents%20To%20Be%20Voted%20On)) 1))))
    (else
      (return (Utilities|Array|Get(acopy) (Variables|VotingSystem|GetEvents%20To%20Be%20Voted%20On) (LocalVariables|GetWinning%20Index))))))

(fn ExecuteDirectorEvent
  (bind _returnvalue (Game|GetPlayerCharacter 0))
  (bind _returnvalue_2 (Math|Random|RandomIntegerinRange 1 3))
  (bind _returnvalue_3 (Math|Random|RandomIntegerinRange 1 4))
  (switch Utilities|FlowControl|Switch|SwitchonDirectorEvents_Enum (Variables|VotingSystem|GetWinning%20Event)
    (:NewEnumerator1
      (Class|AISenseHearing|ReportNoiseEvent (Transformation|GetActorLocation _returnvalue) 1.0 _returnvalue 0.0 "Director")
      (Development|PrintString "Sound played on player"))
    (:NewEnumerator2
      (DirectorEvents|AlertNearestGuard)
      (Development|PrintString "Nearest Guard Alerted"))
    (:NewEnumerator5
      (DirectorEvents|SpawnNGuards _returnvalue_3 false)
      (Development|PrintString (Utilities|String|Append "Spawned " (Utilities|String|ToString(Integer) _returnvalue_3) "Guards") false))
    (:NewEnumerator6
      (DirectorEvents|SpawnNGuards _returnvalue_2 true)
      (Development|PrintString (Utilities|String|Append "Spawned " (Utilities|String|ToString(Integer) _returnvalue_2) "Hunters") false))
    (:NewEnumerator7
      (DirectorEvents|TurnOffGI)
      (Development|PrintString "Lights out!"))
    (:NewEnumerator8
      (DirectorEvents|ShuffleGuardPatrols)
      (Development|PrintString "Patrols Shuffled"))
    (:NewEnumerator9
      (DirectorEvents|LockRandomDoor)
      (Development|PrintString "Locked Random Door"))
    (:NewEnumerator10
      (DirectorEvents|ParanormalActivity)
      (Development|PrintString "Spooky!"))))

(fn AlertNearestGuard
  (bind _outactors (Actor|GetAllActorsOfClass "/Game/Blueprints/Enemies/ALS_Guard_CharacterBP.ALS_Guard_CharacterBP_C"))
  (bind _output_get (LocalVariables|SetGuard%20Array _outactors))
  (for _array_element _output_get
    (if (< (Math|Vector|VectorLength (- (Transformation|GetActorLocation (Variables|Default|GetPlayerCharacter)) (Transformation|GetActorLocation _array_element))) (LocalVariables|GetminDistance))
      (LocalVariables|SetminDistance (Math|Vector|VectorLength (- (Transformation|GetActorLocation (Variables|Default|GetPlayerCharacter)) (Transformation|GetActorLocation _array_element))))
      (LocalVariables|SetClosest%20Guard _array_element)))
  (bind _asguard_ai_controller (Utilities|Casting|CastToGuard_AI_Controller (AI|GetAIController (LocalVariables|GetClosest%20Guard))))
  (Default|BeginSearchingforPlayer _asguard_ai_controller)
  (return))

(fn SpawnNGuards
  (params (Amount%20To%20Spawn :type Integer) (Hunters? :type Boolean))
  (Utilities|FlowControl|Sequence
    (:then_0
      (bind _outactors (Actor|GetAllActorsOfClass "/Game/Blueprints/Enemies/GuardSpawner/GuardSpawner.GuardSpawner_C"))
      (LocalVariables|SetGuard%20Spawners _outactors))
    (:then_1
      (for _index (range 0 Amount%20To%20Spawn)
        (Default|SpawnNGuards (.OutItem (Utilities|Array|Random (LocalVariables|GetGuard%20Spawners))) 1 Hunters?)))))

(fn ShuffleGuardPatrols
  (bind _outactors (Actor|GetAllActorsOfClass "/Game/Blueprints/Enemies/ALS_Guard_CharacterBP.ALS_Guard_CharacterBP_C"))
  (bind _output_get (LocalVariables|SetGuard%20Array _outactors))
  (for _array_element _output_get
    (Utilities|IsValid (Actor|GetComponentbyClass _array_element "/Game/Blueprints/Enemies/AIPatrol_ABP.AIPatrol_ABP_C")
      (:Is%20Valid
        (Default|PopulatePatrolRoute (Actor|GetComponentbyClass _array_element "/Game/Blueprints/Enemies/AIPatrol_ABP.AIPatrol_ABP_C"))
        (return))))
  (Development|PrintString "All Guard Patrols Shuffled"))

(fn ParanormalActivity
  (bind _asals_player_character_bp (Utilities|Casting|CastToALS_Player_CharacterBP (Game|GetPlayerCharacter 0)))
  (Default|ActivateRadialForceforNSeconds _asals_player_character_bp 2.0))

(fn LockRandomDoor
  (bind _outactors (Actor|GetAllActorsOfClass "/Game/Blueprints/Interactables/Props/HingeDoor_BP.HingeDoor_BP_C"))
  (bind _output_get (LocalVariables|SetDoors _outactors))
  (Variables|/Game/Blueprints/Interactables/Props/HingeDoor_BP.HingeDoor_BP_C|SetbIsLocked (.OutItem (Utilities|Array|Random _output_get)) true)
  (return))

(fn ActivateRandomFurniture
  (bind _outactors (Actor|GetAllActorsOfClass "/Game/PolygonOffice/Blueprints/Lighting/ActiveProp_BP.ActiveProp_BP_C"))
  (for _array_element _outactors
    (if (< (Math|Vector|VectorLength (Math|Vector|VectorGetAbs (- (Transformation|GetActorLocation (Game|GetPlayerCharacter 0)) (Transformation|GetActorLocation _array_element)))) (LocalVariables|GetMinDist))
      (LocalVariables|SetClosest%20Active%20Prop _array_element)
      (LocalVariables|SetMinDist (Math|Vector|VectorLength (Math|Vector|VectorGetAbs (- (Transformation|GetActorLocation (Game|GetPlayerCharacter 0)) (Transformation|GetActorLocation _array_element)))))))
  (bind _closest_active_prop (LocalVariables|GetClosest%20Active%20Prop)
    (:then
      (Default|PlayAudio _closest_active_prop))
    (:else)))

(fn TurnOffGI
  (bind _returnvalue (Actor|GetActorOfClass "/Script/Engine.PostProcessVolume"))
  (Utilities|Struct|SetmembersinPostProcessSettings (Variables|/Script/Engine.PostProcessVolume|GetSettings _returnvalue) 0.0)
  (Utilities|Time|SetTimerbyFunctionName 0 "Turn On GI" 15.0))

(fn TurnonGI
  (bind _returnvalue (Actor|GetActorOfClass "/Script/Engine.PostProcessVolume"))
  (Utilities|Struct|SetmembersinPostProcessSettings (Variables|/Script/Engine.PostProcessVolume|GetSettings _returnvalue) 1.0))

(fn ClearAllTimers
  (Utilities|Time|ClearandInvalidateTimerbyHandle (Variables|Default|GetInit%20Votes%20Handle))
  (Utilities|Time|ClearandInvalidateTimerbyHandle (Variables|Default|GetBegin%20Votes%20Handle))
  (Utilities|Time|ClearandInvalidateTimerbyHandle (Variables|Default|GetEnd%20Votes%20Handle)))

(fn SetupConnectandAuthenticate
  (params (OAuthToken :type String) (UserName :type String) (Channel :type String) (Message :type String))
  (bind _twitchirc (Variables|Default|GetTwitchIRC))
  (Class|TwitchIRCComponent|SetupUserInfo _twitchirc OAuthToken UserName Channel)
  (bind _returnvalue (Class|TwitchIRCComponent|Connect _twitchirc))
  (bind _returnvalue_2 (Class|TwitchIRCComponent|Authenticate _twitchirc))
  (if (and _returnvalue_2 _returnvalue)
    (Class|TwitchIRCComponent|SendtoChat _twitchirc Message Channel)))