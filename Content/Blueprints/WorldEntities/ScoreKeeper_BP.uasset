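; ScoreKeeper_BP is a world entity that tracks the run score and owns the on-screen objective widget.
; BeginPlay caches the game instance and creates the objective widget, whose text SetNewObjective updates and which EndPlay removes.
; InitializeMultiplier derives the score modifier from the game instance's starting tokens.
; UpdateScore adds the rounded-up, multiplied delta to the run score and spawns a popup showing the event name and unmultiplied delta.
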(event EventBeginPlay
  (Utilities|FlowControl|Sequence
    (:then_0
      (bind _asci_game_instance_bp (Utilities|Casting|CastToCI_GameInstance_BP (Game|GetGameInstance)))
      (Variables|Default|SetGame%20Instance _asci_game_instance_bp))
    (:then_1
      (bind _returnvalue (UserInterface|CreateWidget "/Game/UI/Objective_Widget.Objective_Widget_C" (Game|GetPlayerController 0)))
      (bind _output_get (Variables|Default|SetObjectiveWidget _returnvalue))
      (UserInterface|Viewport|AddtoViewport _output_get 0))))

(event EventEndPlay
  (params (EndPlayReason :type EEndPlayReason%20Enum :default "Destroyed"))
  (Widget|RemovefromParent (Variables|Default|GetObjectiveWidget)))

(fn ConstructionScript)

(fn UpdateScore
  (params (ScoreDelta :type Integer) (EventName :type String))
  (Variables|Default|SetRun%20Score (+ (Variables|Default|GetRun%20Score) (Math|Float|Ceil (* ScoreDelta (Variables|Default|GetScore%20Modifier)))))
  ;[1 1 1] Spawn Widget with score update
  (bind _returnvalue (UserInterface|CreateWidget "/Game/UI/Score_Update_widget.Score_Update_Widget_C" 0 (Utilities|Text|ToText(String) EventName) ScoreDelta))
  (UserInterface|Viewport|AddtoViewport _returnvalue 1))

(fn InitializeMultiplier
  ;[1 1 1] Add to multiplier based on how many tokens the player has available
  (Variables|Default|SetScore%20Modifier (+ (* (Variables|/Game/Blueprints/GameModes/CI_GameInstance_BP.CI_GameInstance_BP_C|GetStartingTokens (Variables|Default|GetGame%20Instance)) 0.1) 1.0)))

(fn SetNewObjective
  (params (Objective%20Text :type Text))
  (Variables|/Game/UI/Objective_Widget.Objective_Widget_C|SetObjectiveText (Variables|Default|GetObjectiveWidget) Objective%20Text))